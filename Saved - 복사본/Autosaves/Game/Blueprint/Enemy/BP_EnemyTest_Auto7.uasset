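; BP_EnemyTest is a test enemy that takes damage from first-person projectiles and is destroyed when its health runs out.
; On actor overlap it casts the other actor to BP_FirstPersonProjectile, compares it against that class, and subtracts the projectile's Damage from Hp.
; It prints debug strings for the hit and remaining Hp, and destroys itself once Hp reaches zero or below.
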(event EventBeginPlay)

(event EventTick
  (params (DeltaSeconds :type Float%20%28single-precision%29)))

(event Collision|EventActorBeginOverlap
  (params (OtherActor :type Actor%20Object%20Reference))
  (bind _asbp_first_person_projectile (Utilities|Casting|CastToBP_FirstPersonProjectile OtherActor))
  (if (== OtherActor "/Game/Blueprint/Player/BP_FirstPersonProjectile.BP_FirstPersonProjectile")
    (Development|PrintString "hit")
    (Variables|Default|Sethp (- (Variables|Default|Gethp) (Variables|/Game/Blueprint/Player/BP_FirstPersonProjectile.BP_FirstPersonProjectile_C|Getdamage _asbp_first_person_projectile)))
    (if (<= (Variables|Default|Gethp) 0)
      (Actor|DestroyActor)
      (else
        (Development|PrintString (Utilities|String|ToString(Integer) (Variables|Default|Gethp)))))))

(fn ConstructionScript)